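; Interactive hinged door that the first-person player opens away from or closes with the Interact input.
; Left and right entrance triggers enable input, record the player's side and print a prompt, disabling input on exit.
; Two timelines rotate the hinge forward or backward and play in reverse to close, with input locked during movement.
; When each finishes, the door state updates and a blocker's collision is enabled only while closed.
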(event `self.Left Entrance.OnComponentBeginOverlap`
  (params (OverlappedComponent :type "PrimitiveComponent Object Reference") (OtherActor :type "Actor Object Reference") (OtherComp :type "PrimitiveComponent Object Reference") (OtherBodyIndex :type Integer) (bFromSweep :type Boolean) (SweepResult :type "HitResult Structure (by ref)"))
  ;[1 1 1] Checks if the player is able to interact with the door.
  (`self.AllowInteraction` OtherActor true))

(event `self.Right Entrance.OnComponentBeginOverlap`
  (params (OverlappedComponent :type "PrimitiveComponent Object Reference") (OtherActor :type "Actor Object Reference") (OtherComp :type "PrimitiveComponent Object Reference") (OtherBodyIndex :type Integer) (bFromSweep :type Boolean) (SweepResult :type "HitResult Structure (by ref)"))
  ;[1 1 1] Checks if the player is able to interact with the door.
  (`self.AllowInteraction` OtherActor))

(event `self.Left Entrance.OnComponentEndOverlap`
  (params (OverlappedComponent :type "PrimitiveComponent Object Reference") (OtherActor :type "Actor Object Reference") (OtherComp :type "PrimitiveComponent Object Reference") (OtherBodyIndex :type Integer))
  ;[1 1 1] Checks if the player is able to interact with the door.
  (`self.DisablePlayerInput` OtherActor))

(event `self.Right Entrance.OnComponentEndOverlap`
  (params (OverlappedComponent :type "PrimitiveComponent Object Reference") (OtherActor :type "Actor Object Reference") (OtherComp :type "PrimitiveComponent Object Reference") (OtherBodyIndex :type Integer))
  ;[1 1 1] Checks if the player is able to interact with the door.
  (`self.DisablePlayerInput` OtherActor))

(event `InputAction|Interact`
  (params (Key :type "Key Structure"))
  (bind _hinge (`self.Hinge`))
  ;[1 1 1] Opens or closes the door depending on the state of the door and what side of the door the player is on.
  (:`Pressed`
    (`TimelineComponent.SetPlayRate` (`self.Open Door Backward`) (`self.playRate`))
    (`TimelineComponent.SetPlayRate` (`self.Open Door Forward`) (`self.playRate`))
    (`self.DisableInput` (`GameplayStatics.GetPlayerController` 0))
    (switch `string` (`self.state`)
      (:`Opened Forward`
        (bind (_direction _open_door_forward) (`Timeline|Open Door Forward` :!via `ReverseFromEnd` :!label _label)
          (:`Update`
            (`SceneComponent.K2_SetRelativeRotation` _hinge (`KismetMathLibrary.MakeRotator` 0.0 0.0 _open_door_forward) false false))
          (:`Finished`
            (`self.Set Door State` _open_door_forward "Opened Forward")
            (`self.EnableInput` (`GameplayStatics.GetPlayerController` 0) :!label _label_2))))
      (:`Closed`
        (if (`self.inFrontOfDoor`)
          (goto _label :!via `PlayFromStart`)
          (else
            (bind (_direction_2 _open_door_backward) (`Timeline|Open Door Backward` :!via `PlayFromStart` :!label _label_3)
              (:`Update`
                (`SceneComponent.K2_SetRelativeRotation` _hinge (`KismetMathLibrary.MakeRotator` 0.0 0.0 _open_door_backward) false false))
              (:`Finished`
                (`self.Set Door State` _open_door_backward "Opened Backward")
                (goto _label_2))))))
      (:`Opened Backward`
        (goto _label_3 :!via `ReverseFromEnd`)))))

(fn `AllowInteraction`
  (params (Object :type "Object Object Reference") (InFrontOfDoor :type Boolean))
  (cast `/Game/Blueprints/Actors/FirstPersonCharacter` Object)
  (set `self.inFrontOfDoor` InFrontOfDoor)
  (`self.EnableInput` (`GameplayStatics.GetPlayerController` 0))
  (if (`KismetStringLibrary.EqualEqual_StrStr` (`self.state`) "Closed")
    (`KismetSystemLibrary.PrintString` "Press \"E\" to open.")
    (else
      (`KismetSystemLibrary.PrintString` "Press \"E\" to close."))))

(fn `DisablePlayerInput`
  (params (Object :type "Object Object Reference"))
  (cast `/Game/Blueprints/Actors/FirstPersonCharacter` Object)
  (`self.DisableInput` (`GameplayStatics.GetPlayerController` 0)))

(fn `Set Door State`
  (params (hingeRotation :type "Float (double-precision)") (altDoorState :type String))
  (bind _blocker (`self.Blocker`))
  (if (== hingeRotation 0.0)
    (set `self.state` "Closed")
    (`PrimitiveComponent.SetCollisionEnabled` _blocker "QueryAndPhysics")
    (else
      (set `self.state` altDoorState)
      (`PrimitiveComponent.SetCollisionEnabled` _blocker "NoCollision"))))

(fn `UserConstructionScript`)
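; Elevator actor that rises and descends on Turnon and TurnOff signals, such as from linked switches or a pressure plate.
; The construction script sets travel height from the floor count and builds shaft walls per floor as instanced meshes, leaving openings at bottom and top.
; A timeline, rate-scaled by velocity over height, moves the platform.
; On finish it clears the activators' in-progress flags and flip-flops the Up state.
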(event `self.ReceiveBeginPlay`
  ;[1 1 1] Adjusts the play rate depending on the elevator's velocity and maximum height.
  (`TimelineComponent.SetPlayRate` (`self.AnimElevate`) (/ (`self.Velocity`) (`self.MaxHeight`))))

(event `/Game/Blueprints/Interfaces/ToggleableObject.Turn On`
  (params (Player :type "/Game/Blueprints/Actors/FirstPersonCharacter Object Reference"))
  ;[1 1 1] Sends the elevator up when turned on and down when turned off while returning its current state to its activator.
  (bind (_direction _percent) (`Timeline|AnimElevate` :!via `PlayFromStart` :!label _label)
    (:`Update`
      (`SceneComponent.K2_SetRelativeLocation` (`self.Mover`) (`KismetMathLibrary.MakeVector` 0.0 0.0 (* _percent (`self.MaxHeight`))) false false))
    (:`Finished`
      (bind _asswitch (cast `/Game/Blueprints/Actors/Switch` (`self.switch1`))
        (:`then`
          (set `/Game/Blueprints/Actors/Switch.eventInProgress` false _asswitch)
          (bind _asswitch_2 (cast `/Game/Blueprints/Actors/Switch` (`self.switch2`))
            (:`then`
              (set `/Game/Blueprints/Actors/Switch.eventInProgress` false _asswitch_2))
            (:`CastFailed`
              _)))
        (:`CastFailed`
          _))
      (bind _aspressure_plate (cast `/Game/Blueprints/Actors/PressurePlate` (`self.plate`))
        (:`then`
          (set `/Game/Blueprints/Actors/PressurePlate.eventInProgress` false _aspressure_plate))
        (:`CastFailed`
          _))
      (`/Engine/EditorBlueprintResources/StandardMacros.FlipFlop`
        (:`A`
          (set `self.up` true))
        (:`B`
          (set `self.up` false))))))

(event `/Game/Blueprints/Interfaces/ToggleableObject.Turn Off`
  (params (Player :type "/Game/Blueprints/Actors/FirstPersonCharacter Object Reference"))
  ;[1 1 1] Sends the elevator up when turned on and down when turned off while returning its current state to its activator.
  (goto _label :!via `ReverseFromEnd`))

(fn `UserConstructionScript`
  (locals (currentFloor :type Integer) (`current Z` :type "Float (double-precision)"))
  (bind _wallinstancemesh (`self.WallInstanceMesh`))
  (bind _current_z (`local.current Z`))
  (set `self.MaxHeight` (* (`self.maxFloors`) 400.0))
  (for _index (range (+ (`self.maxFloors`) 1))
    (bind _output_get (set `local.currentFloor` _index))
    (set `local.current Z` (* _output_get 400.0))
    (`InstancedStaticMeshComponent.AddInstance` _wallinstancemesh (`KismetMathLibrary.MakeTransform` (`KismetMathLibrary.MakeVector` -200.0 210.0 _current_z)))
    (`InstancedStaticMeshComponent.AddInstance` _wallinstancemesh (`KismetMathLibrary.MakeTransform` (`KismetMathLibrary.MakeVector` -200.0 -210.0 _current_z)))
    (if (!= (`local.currentFloor`) (`self.maxFloors`))
      (`InstancedStaticMeshComponent.AddInstance` _wallinstancemesh (`KismetMathLibrary.MakeTransform` (`KismetMathLibrary.MakeVector` 210.0 -200.0 _current_z) (struct :`Yaw` 90.0)))
      (if (!= (`local.currentFloor`) 0)
        (`InstancedStaticMeshComponent.AddInstance` _wallinstancemesh (`KismetMathLibrary.MakeTransform` (`KismetMathLibrary.MakeVector` -190.0 -200.0 _current_z) (struct :`Yaw` 90.0)))))))
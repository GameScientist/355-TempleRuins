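; Rideable physics hoverboard that the player possesses by interacting, destroying their character, and leaves by spawning a new FirstPersonCharacter above it.
; The construction script sizes the board from Length and Width and builds eight corner arrow thrusters, four downward and four angled.
; Each tick, thrusters line-trace and push opposite the ray, with force scaling up with hit distance.
; Input axes add forward force and yaw torque; the ground-normal ApplyTorque is never called here.
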(event `self.ReceiveTick`
  (params (DeltaSeconds :type "Float (single-precision)"))
  (`self.ThrustAll` DeltaSeconds)
  (`self.ThrustAt` (0.0 0.0 0.0) (0.0 0.0 0.0) DeltaSeconds))

(event `/Game/Blueprints/Interfaces/PlayerWantsToInteract.PlayerWantsToInteract`
  (params (Player :type "/Game/Blueprints/Actors/FirstPersonCharacter Object Reference"))
  (`Controller.Possess` (`self.GetController` Player) self)
  (`self.K2_DestroyActor` Player))

(event `InputAction|Interact`
  (params (Key :type "Key Structure"))
  (:`Pressed`
    (bind _returnvalue (`|SpawnActorFromClass` "/Game/Blueprints/Actors/FirstPersonCharacter.FirstPersonCharacter_C" (`KismetMathLibrary.MakeTransform` (+ (`SceneComponent.K2_GetComponentLocation` (`self.Root`)) (0.0 0.0 50.0)) (`KismetMathLibrary.MakeRotator` 0.0)) "Undefined" "OverrideRootScale" null null))
    (`Controller.Possess` (`self.GetController`) _returnvalue)))

(event `InputAxis|MoveForward`
  (params (AxisValue :type "Float (single-precision)"))
  (bind _root (`self.Root`))
  (`PrimitiveComponent.AddForce` _root (* (`SceneComponent.GetForwardVector` _root) (* AxisValue (`self.acceleration`))) "None" true))

(event `InputAxis|MoveRight`
  (params (AxisValue :type "Float (single-precision)"))
  (bind _root (`self.Root`))
  (`PrimitiveComponent.AddTorqueInRadians` _root (* (`SceneComponent.GetUpVector` _root) (* AxisValue (`self.acceleration`))) "None" false))

(fn `ApplyTorque`
  (params (B :type "Float (double-precision)"))
  (bind _root (`self.Root`))
  (set `self.groundNormal` (/ (`self.groundNormal`) (`KismetMathLibrary.Conv_IntToDouble` (`KismetArrayLibrary.Array_Length` (`self.thrusters`)))))
  (`PrimitiveComponent.AddTorqueInRadians` _root (* (`KismetMathLibrary.Cross_VectorVector` (`SceneComponent.GetUpVector` _root) (`self.groundNormal`)) (* (`self.torqueAmount`) B)) "None" true)
  (set `self.groundNormal` (0.0 0.0 0.0)))

(fn `ThrustAll`
  (params (DT :type "Float (double-precision)"))
  (for _array_element (`self.thrusters`)
    (`self.ThrustAt` (`SceneComponent.K2_GetComponentLocation` _array_element) (`SceneComponent.GetForwardVector` _array_element) DT)))

(fn `ThrustAt`
  (params (`World Output` :type "Vector Structure") (Dir :type "Vector Structure") (DT :type "Float (double-precision)"))
  (bind (_outhit _returnvalue) (`KismetSystemLibrary.LineTraceSingle` :`Start` `World Output` :`End` (+ `World Output` (* Dir (`self.rayLength`))) :`TraceChannel` "TraceTypeQuery1" :`DrawDebugType` "ForOneFrame"))
  (if _returnvalue
    (bind (_bblockinghit _binitialoverlap _time _distance _location _impactpoint _normal _impactnormal) (`GameplayStatics.BreakHitResult` _outhit))
    (`PrimitiveComponent.AddForceAtLocation` (`self.Root`) (* (`local.Dir`) (* (/ _distance 1000.0) (`self.thrustAmount`) -1.0 DT)) (`local.World Output`) "None")
    (set `self.groundNormal` (+ _impactnormal (0.0 0.0 0.0)))
    (else
      (set `self.groundNormal` (+ _impactnormal (0.0 0.0 1.0))))))

(fn `UserConstructionScript`
  (bind _length (`self.length`))
  (bind _width (`self.width`))
  (bind _length_2 (`self.length`))
  (bind _width_2 (`self.width`))
  (`SceneComponent.SetRelativeScale3D` (`self.Cube`) (`KismetMathLibrary.MakeVector` (/ _length_2 100.0) (/ _width_2 100.0) 0.2))
  (bind _returnvalue (`AddComponent|NODE_AddArrowComponent-0` :`RelativeTransform` (`KismetMathLibrary.MakeTransform` (`KismetMathLibrary.MakeVector` (/ _length_2 2.0) (/ _width_2 2.0) -60.0) (struct :`Pitch` -90.0 :`Yaw` -90.0))))
  (bind _returnvalue_2 (`AddComponent|NODE_AddArrowComponent-1` :`RelativeTransform` (`KismetMathLibrary.MakeTransform` (`KismetMathLibrary.MakeVector` (/ _length_2 2.0) (/ _width_2 -2.0) -60.0) (struct :`Pitch` -90.0 :`Yaw` -90.0))))
  (bind _returnvalue_3 (`AddComponent|NODE_AddArrowComponent-2` :`RelativeTransform` (`KismetMathLibrary.MakeTransform` (`KismetMathLibrary.MakeVector` (/ _length_2 -2.0) (/ _width_2 2.0) -60.0) (struct :`Pitch` -90.0 :`Yaw` -90.0))))
  (bind _returnvalue_4 (`AddComponent|NODE_AddArrowComponent-3` :`RelativeTransform` (`KismetMathLibrary.MakeTransform` (`KismetMathLibrary.MakeVector` (/ _length_2 -2.0) (/ _width_2 -2.0) -60.0) (struct :`Pitch` -90.0 :`Yaw` -90.0))))
  (`SceneComponent.SetRelativeScale3D` (`self.Cube`) (`KismetMathLibrary.MakeVector` (/ _length 100.0) (/ _width 100.0) 0.2))
  (bind _returnvalue_5 (`AddComponent|NODE_AddArrowComponent-4` :`RelativeTransform` (`KismetMathLibrary.MakeTransform` (`KismetMathLibrary.MakeVector` (/ _length 2.0) (/ _width 2.0) -60.0) (struct :`Pitch` -135.0 :`Yaw` -135.0))))
  (bind _returnvalue_6 (`AddComponent|NODE_AddArrowComponent-5` :`RelativeTransform` (`KismetMathLibrary.MakeTransform` (`KismetMathLibrary.MakeVector` (/ _length 2.0) (/ _width -2.0) -60.0) (struct :`Pitch` -135.0 :`Yaw` 135.0))))
  (bind _returnvalue_7 (`AddComponent|NODE_AddArrowComponent-6` :`RelativeTransform` (`KismetMathLibrary.MakeTransform` (`KismetMathLibrary.MakeVector` (/ _length -2.0) (/ _width 2.0) -60.0) (struct :`Pitch` -135.0 :`Yaw` -45.0))))
  (bind _returnvalue_8 (`AddComponent|NODE_AddArrowComponent-7` :`RelativeTransform` (`KismetMathLibrary.MakeTransform` (`KismetMathLibrary.MakeVector` (/ _length -2.0) (/ _width -2.0) -60.0) (struct :`Pitch` -135.0 :`Yaw` 45.0))))
  (set `self.thrusters` (`|MakeArray` _returnvalue _returnvalue_2 _returnvalue_3 _returnvalue_4 _returnvalue_5 _returnvalue_6 _returnvalue_7 _returnvalue_8)))
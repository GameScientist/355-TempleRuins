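; Pressure plate actor that toggles a linked Door2 or Elevator when the first-person character steps on it.
; Overlap plays a timeline that lowers the slab; once fully pushed, it sets EventInProgress and sends TurnOn or TurnOff based on the device's state.
; EventFinished reverses the timeline only if the plate is pushed and no longer weighed down.
; Stepping off only clears the weighed-down flag.
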(event `self.Collision.OnComponentBeginOverlap`
  (params (OverlappedComponent :type "PrimitiveComponent Object Reference") (OtherActor :type "Actor Object Reference") (OtherComp :type "PrimitiveComponent Object Reference") (OtherBodyIndex :type Integer) (bFromSweep :type Boolean) (SweepResult :type "HitResult Structure (by ref)"))
  (bind _other (`self.Other`))
  ;[1 1 1 1 12] When the player steps on the pressure plate, it is pushed down, and then signals a device to be turned on or off.
  ;;[1 1 1 1 12] The slab will move down when the player is on top of it, and pop back out when the player moves off of it and the triggered event is finished.
  (cast `/Game/Blueprints/Actors/FirstPersonCharacter` OtherActor)
  (set `self.weighedDown` true)
  (if (not (`self.eventInProgress`))
    (bind (_direction _height) (`Timeline|PlatePush` :!label _label)
      (:`Update`
        ;;[1 1 1 1 12] The slab is pressed down until it reaches a certain point, then signals a device to be turned on or off.
        (set `self.pushed` (== _height -25.0))
        (`SceneComponent.K2_SetRelativeLocation` (`self.Slab`) (`KismetMathLibrary.MakeVector` 0.0 0.0 _height) false false))
      (:`Finished`
        (if (`self.pushed`)
          (set `self.eventInProgress` true)
          (bind _asdoor_2 (cast `/Game/Blueprints/Actors/Door2` _other)
            (:`then`
              (if (`/Game/Blueprints/Actors/Door2.open` _asdoor_2)
                (message `/Game/Blueprints/Interfaces/ToggleableObject.Turn Off` _other null :!label _label_2)
                (else
                  (message `/Game/Blueprints/Interfaces/ToggleableObject.Turn On` _other null :!label _label_3))))
            (:`CastFailed`
              (bind _aselevator (cast `/Game/Blueprints/Actors/Elevator` _other))
              (if (`/Game/Blueprints/Actors/Elevator.up` _aselevator)
                (goto _label_2)
                (else
                  (goto _label_3))))))))))

(event `EventFinished`
  ;[1 1 1 1 12] When the player steps on the pressure plate, it is pushed down, and then signals a device to be turned on or off.
  ;;[1 1 1 1 12] The slab will move down when the player is on top of it, and pop back out when the player moves off of it and the triggered event is finished.
  (if (and (not (`self.weighedDown`)) (`self.pushed`))
    (goto _label :!via `Reverse`)))

(event `self.Collision.OnComponentEndOverlap`
  (params (OverlappedComponent :type "PrimitiveComponent Object Reference") (OtherActor :type "Actor Object Reference") (OtherComp :type "PrimitiveComponent Object Reference") (OtherBodyIndex :type Integer))
  ;[1 1 1] The pressure plate detects when it is no longer being stepped on.
  (cast `/Game/Blueprints/Actors/FirstPersonCharacter` OtherActor)
  (set `self.weighedDown` false))

(fn `UserConstructionScript`)
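; TriggerButton is a pressable button actor that switches a linked Device, a door or elevator, on or off.
; PushButton runs the Insert timeline to slide the button in, then sets EventInProgress and sends TurnOn or TurnOff based on the Device's cast state.
; Tick reverses the timeline once EventInProgress is cleared.
; Separately, PlayerWantstoInteract sends TriggerMessage to every Triggerable in ObjectsToTrigger.
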(event `PushButton`
  (bind _device (`self.device`))
  ;[1 1 1 1 12] The button is pushed in when interacted with and pops back out when the object event is finished, allowing the player to press the button again.
  (if (not (`self.eventInProgress`))
    (bind (_direction _insert) (`Timeline|Insert` :!via `PlayFromStart` :!label _label)
      (:`Update`
        ;[1 1 1] The button is pushed down until it reaches a certain point, at which point it toggles an object on or off.
        (set `self.pushed` (== _insert -25.0))
        (`SceneComponent.K2_SetRelativeLocation` (`self.Button`) (`KismetMathLibrary.MakeVector` _insert) false false))
      (:`Finished`
        (if (`self.pushed`)
          (set `self.eventInProgress` true)
          (bind _asdoor_2 (cast `/Game/Blueprints/Actors/Door2` _device)
            (:`then`
              (if (`/Game/Blueprints/Actors/Door2.open` _asdoor_2)
                (message `/Game/Blueprints/Interfaces/ToggleableObject.Turn Off` _device null :!label _label_2)
                (else
                  (message `/Game/Blueprints/Interfaces/ToggleableObject.Turn On` _device null :!label _label_3))))
            (:`CastFailed`
              (bind _aselevator (cast `/Game/Blueprints/Actors/Elevator` _device))
              (if (`/Game/Blueprints/Actors/Elevator.up` _aselevator)
                (goto _label_2)
                (else
                  (goto _label_3))))))))))

(event `self.ReceiveTick`
  (params (DeltaSeconds :type "Float (single-precision)"))
  ;[1 1 1 1 12] The button is pushed in when interacted with and pops back out when the object event is finished, allowing the player to press the button again.
  (if (and (not (`self.eventInProgress`)) (`self.pushed`))
    (goto _label :!via `ReverseFromEnd`)))

(event `/Game/Blueprints/Interfaces/PlayerWantsToInteract.PlayerWantsToInteract`
  (params (Player :type "/Game/Blueprints/Actors/FirstPersonCharacter Object Reference"))
  (for _array_element (`self.objectsToTrigger`)
    (if (`KismetSystemLibrary.DoesImplementInterface` _array_element "/Game/Blueprints/Interfaces/Triggerable.Triggerable_C")
      (message `/Game/Blueprints/Interfaces/Triggerable.Trigger` _array_element))))

(event `OpenTheDoor`)

(fn `UserConstructionScript`)
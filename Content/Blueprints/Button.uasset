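; Push button that can activate once and toggles a message on a linked Door2 actor based on whether it is open.
; PushButton plays the Insert timeline, which slides the Cylinder along local X, and Tick reverses it at full depth while not yet activated.
; When the timeline finishes fully pressed, it sets Activated and casts Other to Door2 to turn the message off if open, on otherwise.
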(event `self.ReceiveTick`
  (params (DeltaSeconds :type "Float (single-precision)"))
  (bind _other (`self.Other`))
  (bind _returnvalue (== (stale _insert) -25.0))
  (if (and (not (`self.Activated`)) _returnvalue)
    (bind (_direction _insert) (`Timeline|Insert` :!via `ReverseFromEnd` :!label _label)
      (:`Update`
        (`SceneComponent.K2_SetRelativeLocation` (`self.Cylinder`) (`KismetMathLibrary.MakeVector` _insert) false false))
      (:`Finished`
        (if _returnvalue
          (set `self.activated` true)
          (bind _asdoor_2 (cast `/Game/Blueprints/Door2` _other))
          (if (`/Game/Blueprints/Door2.open` _asdoor_2)
            (message `/Game/Blueprints/ToggleableObject.Turn Off` _other null)
            (else
              (message `/Game/Blueprints/ToggleableObject.Turn On` _other null))))))))

(event `PushButton`
  (if (not (`self.Activated`))
    (goto _label :!via `PlayFromStart`)))

(fn `UserConstructionScript`)
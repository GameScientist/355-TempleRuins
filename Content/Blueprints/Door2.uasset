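; Sliding double door that opens on a Turnon event and closes on TurnOff.
; The OpenDoors timeline plays or reverses to move the left and right panels along relative X at a fixed height.
; When the timeline finishes, it clears Activated on the referenced Button and PressurePlate, and a FlipFlop toggles the Open flag.
; Player interaction and input-disabling calls remain in the graph but are unconnected.
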(event `/Game/Blueprints/ToggleableObject.Turn On`
  (params (Player :type "/Game/Blueprints/FirstPersonCharacter Object Reference"))
  (bind (_direction _left_door_open _right_door_open) (`Timeline|OpenDoors` :!label _label)
    (:`Update`
      (`SceneComponent.K2_SetRelativeLocation` (`self.Left Door`) (`KismetMathLibrary.MakeVector` _left_door_open 0.0 105.0) false false)
      (`SceneComponent.K2_SetRelativeLocation` (`self.Right Door`) (`KismetMathLibrary.MakeVector` _right_door_open 0.0 105.0) false false))
    (:`Finished`
      (bind _asbutton (cast `/Game/Blueprints/Button` (`self.button`))
        (:`then`
          (set `/Game/Blueprints/Button.Activated` false _asbutton))
        (:`CastFailed`
          _))
      (bind _aspressure_plate (cast `/Game/Blueprints/PressurePlate` (`self.plate`))
        (:`then`
          (set `/Game/Blueprints/PressurePlate.activated` false _aspressure_plate))
        (:`CastFailed`
          _))
      (`/Engine/EditorBlueprintResources/StandardMacros.FlipFlop`
        (:`A`
          (set `self.open` true))
        (:`B`
          (set `self.open` false))))))

(event `/Game/Blueprints/ToggleableObject.Turn Off`
  (params (Player :type "/Game/Blueprints/FirstPersonCharacter Object Reference"))
  (goto _label :!via `Reverse`))

(fn `UserConstructionScript`)
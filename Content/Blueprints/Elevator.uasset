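; Elevator actor that carries its Mover from the bottom to the top of a procedurally built shaft.
; The construction script derives height from MaxFloors and places instanced walls per floor, leaving openings at the bottom and top.
; Interact input, enabled while the first-person character overlaps Collider, or PlayerWantstoInteract plays a timeline that raises Mover, rate-scaled by Velocity over height.
; It has no downward travel, and SendElevatorUp is empty.
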(event `self.ReceiveBeginPlay`
  (`TimelineComponent.SetPlayRate` (`self.AnimElevate`) (/ (`self.Velocity`) (`self.MaxHeight`))))

(event `InputAction|Interact`
  (params (Key :type "Key Structure"))
  (:`Pressed`
    (`KismetSystemLibrary.PrintString` "1" :!label _label)
    (bind (_direction _percent) (`Timeline|AnimElevate`)
      (:`Update`
        (`SceneComponent.K2_SetRelativeLocation` (`self.Mover`) (`KismetMathLibrary.MakeVector` 0.0 0.0 (* _percent (`self.MaxHeight`))) false false)))))

(event `SendElevatorUp`)

(event `/Game/Blueprints/PlayerWantsToInteract.PlayerWantsToInteract`
  (params (Player :type "/Game/Blueprints/FirstPersonCharacter Object Reference"))
  (goto _label))

(event `self.Collider.OnComponentBeginOverlap`
  (params (OverlappedComponent :type "PrimitiveComponent Object Reference") (OtherActor :type "Actor Object Reference") (OtherComp :type "PrimitiveComponent Object Reference") (OtherBodyIndex :type Integer) (bFromSweep :type Boolean) (SweepResult :type "HitResult Structure (by ref)"))
  ;[1 1 1] Enables and disables player input.
  (cast `/Game/Blueprints/FirstPersonCharacter` OtherActor)
  (`self.EnableInput` (`GameplayStatics.GetPlayerController` 0)))

(event `self.Collider.OnComponentEndOverlap`
  (params (OverlappedComponent :type "PrimitiveComponent Object Reference") (OtherActor :type "Actor Object Reference") (OtherComp :type "PrimitiveComponent Object Reference") (OtherBodyIndex :type Integer))
  ;[1 1 1] Enables and disables player input.
  (cast `/Game/Blueprints/FirstPersonCharacter` OtherActor)
  (`self.DisableInput` (`GameplayStatics.GetPlayerController` 0)))

(fn `UserConstructionScript`
  (locals (currentFloor :type Integer) (`current Z` :type "Float (double-precision)"))
  (bind _wallinstancemesh (`self.WallInstanceMesh`))
  (bind _current_z (`local.current Z`))
  (set `self.MaxHeight` (* (`self.maxFloors`) 400.0))
  (for _index (range (+ (`self.maxFloors`) 1))
    (bind _output_get (set `local.currentFloor` _index))
    (set `local.current Z` (* _output_get 400.0))
    (`InstancedStaticMeshComponent.AddInstance` _wallinstancemesh (`KismetMathLibrary.MakeTransform` (`KismetMathLibrary.MakeVector` -200.0 210.0 _current_z)))
    (`InstancedStaticMeshComponent.AddInstance` _wallinstancemesh (`KismetMathLibrary.MakeTransform` (`KismetMathLibrary.MakeVector` -200.0 -210.0 _current_z)))
    (if (!= (`local.currentFloor`) (`self.maxFloors`))
      (`InstancedStaticMeshComponent.AddInstance` _wallinstancemesh (`KismetMathLibrary.MakeTransform` (`KismetMathLibrary.MakeVector` 210.0 -200.0 _current_z) (struct :`Yaw` 90.0)))
      (if (!= (`local.currentFloor`) 0)
        (`InstancedStaticMeshComponent.AddInstance` _wallinstancemesh (`KismetMathLibrary.MakeTransform` (`KismetMathLibrary.MakeVector` -190.0 -200.0 _current_z) (struct :`Yaw` 90.0)))))))
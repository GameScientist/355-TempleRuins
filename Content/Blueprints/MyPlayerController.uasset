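; Player controller that creates the player's HUD widget and relays player details to it.
; On BeginPlay it caches the MyGameInstance, adds a new HUD to the viewport and prints a debug greeting.
; A custom UpdateTheHUD event passes the game instance's PlayerDetails to the HUD if it is valid.
; When destroyed, it removes a valid HUD from its parent.
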(event `self.ReceiveBeginPlay`
  (bind _asmy_game_instance (cast `/Game/Blueprints/MyGameInstance` (`GameplayStatics.GetGameInstance`)))
  (set `self.theGameInstance` _asmy_game_instance)
  (bind _returnvalue (`|CreateWidget` "/Game/Blueprints/HUD.HUD_C"))
  (`UserWidget.AddToViewport` _returnvalue 0)
  (`KismetSystemLibrary.PrintString` "Hello"))

(event `UpdateTheHUD`
  (bind _hud (`self.HUD`))
  (`/Engine/EditorBlueprintResources/StandardMacros.IsValid` _hud
    (:`Is Valid`
      (`/Game/Blueprints/HUD.Update the HUD` _hud false (`/Game/Blueprints/MyGameInstance.playerDetails` (`self.theGameInstance`))))))

(event `self.ReceiveDestroyed`
  (bind _hud (`self.HUD`))
  (`/Engine/EditorBlueprintResources/StandardMacros.IsValid` _hud
    (:`Is Valid`
      (`Widget.RemoveFromParent` _hud))))

(fn `UserConstructionScript`)
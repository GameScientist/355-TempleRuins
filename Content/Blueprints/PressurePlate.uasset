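; Pressure plate that the first-person character triggers once to toggle a linked door.
; Collision overlaps track Pushed and play the PlatePush timeline, which drives the plate's relative Z.
; Finishing at the pressed height latches Activated, then sends Other a turn-on or turn-off message based on its Door2 Open state.
; Tick reverses the timeline only when the plate is unlatched, unoccupied and exactly at that height.
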(event `self.ReceiveTick`
  (params (DeltaSeconds :type "Float (single-precision)"))
  (bind _other (`self.Other`))
  (if (and (not (`self.activated`)) (== (stale _height) -25.0) (not (`self.pushed`)))
    (bind (_direction _height) (`Timeline|PlatePush` :!via `Reverse` :!label _label)
      (:`Update`
        (`SceneComponent.K2_SetRelativeLocation` (`self.Pressure Plate`) (`KismetMathLibrary.MakeVector` 0.0 0.0 _height) false false))
      (:`Finished`
        (if (== _height -25.0)
          (set `self.activated` true)
          (bind _asdoor_2 (cast `/Game/Blueprints/Door2` _other))
          (if (`/Game/Blueprints/Door2.open` _asdoor_2)
            (message `/Game/Blueprints/ToggleableObject.Turn Off` _other null)
            (else
              (message `/Game/Blueprints/ToggleableObject.Turn On` _other null))))))))

(event `self.Collision.OnComponentBeginOverlap`
  (params (OverlappedComponent :type "PrimitiveComponent Object Reference") (OtherActor :type "Actor Object Reference") (OtherComp :type "PrimitiveComponent Object Reference") (OtherBodyIndex :type Integer) (bFromSweep :type Boolean) (SweepResult :type "HitResult Structure (by ref)"))
  (cast `/Game/Blueprints/FirstPersonCharacter` OtherActor)
  (set `self.pushed` true)
  (if (not (`self.activated`))
    (goto _label)))

(event `self.Collision.OnComponentEndOverlap`
  (params (OverlappedComponent :type "PrimitiveComponent Object Reference") (OtherActor :type "Actor Object Reference") (OtherComp :type "PrimitiveComponent Object Reference") (OtherBodyIndex :type Integer))
  (cast `/Game/Blueprints/FirstPersonCharacter` OtherActor)
  (set `self.pushed` false))

(fn `UserConstructionScript`)
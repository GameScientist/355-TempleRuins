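; Slime pawn that chases the player by continually pathfinding toward them.
; BeginPlay caches the FirstPersonCharacter actor, then PathfindToPlayer issues an AI MoveTo to its current location and re-calls itself on success or failure.
; Tick also calls PathfindToPlayer every frame, and again through a state-enum switch whose only shown case has an always-true branch.
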(event `self.ReceiveBeginPlay`
  (bind _returnvalue (`GameplayStatics.GetActorOfClass` "/Game/Blueprints/Actors/FirstPersonCharacter.FirstPersonCharacter_C"))
  (set `self.player` _returnvalue)
  (`self.PathfindToPlayer`))

(event `PathfindToPlayer`
  (bind _player (`self.player`))
  (`/Engine/EditorBlueprintResources/StandardMacros.IsValid` _player
    (:`Is Valid`
      (`|AIMoveTo` (`self.GetController`) self (`self.K2_GetActorLocation` _player) null
        (:`OnSuccess`
          _)
        (:`OnFail`
          _))
      (`self.PathfindToPlayer`))))

(event `self.ReceiveTick`
  (params (DeltaSeconds :type "Float (single-precision)"))
  (`self.PathfindToPlayer`)
  (switch `/Game/Blueprints/SlimeStates` "SlimeStates_MAX"
    (:`NewEnumerator0`
      (if true
        (`self.PathfindToPlayer`)))))

(fn `UserConstructionScript`)